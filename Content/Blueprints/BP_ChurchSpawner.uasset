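; BP_ChurchSpawner is an actor that spawns a BP_Church in front of itself when its SpawnChurch event is called.
; The spawn point sits a fixed distance along the root component's forward vector with a vertical lift, and the church takes the spawner's rotation.
; Collision handling nudges the church to fit or skips the spawn if it would still collide; BeginPlay, overlap and Tick do nothing.
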(event Custom|SpawnChurch
  (bind _returnvalue (Transformation|GetActorLocation))
  (bind _defaultsceneroot (Variables|Default|GetDefaultSceneRoot))
  (bind _returnvalue_2 (Math|Vector|GetForwardVector _defaultsceneroot))
  (bind _returnvalue_3 (* _returnvalue_2 400))
  (bind _returnvalue_4 (+ _returnvalue _returnvalue_3))
  (bind (_x _y _z) (Math|Vector|BreakVector _returnvalue_4))
  (Game|SpawnActorfromClass "/Game/Blueprints/BP_Church.BP_Church_C" (Math|Transform|MakeTransform (Math|Vector|MakeVector _x _y (+ _z 8e+01)) (Transformation|GetActorRotation) "1,1,1") "AdjustIfPossibleButDontSpawnIfColliding" 0 0))

(event EventBeginPlay)

(event Collision|EventActorBeginOverlap
  (params (OtherActor :type Actor%20Object%20Reference)))

(event EventTick
  (params (DeltaSeconds :type Float%20%28single-precision%29)))

(fn ConstructionScript)