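; BP_Basilica is a cathedral actor that registers with the player and spawns a Pope.
; On BeginPlay it increments the player character's Popechurches count, stopping if the cast to BP_Character fails.
; It also spawns a BP_Pope in front of the Chathedral component, sets itself as its PatrolPathBasilica and prints a debug message.
; The construction script gives the cathedral a green dynamic material instance.
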(event EventBeginPlay
  (bind _chathedral (Variables|Default|GetChathedral))
  (Utilities|FlowControl|Sequence
    (:then_0
      (bind _asbp_character (Utilities|Casting|CastToBP_Character (Game|GetPlayerCharacter 0)))
      (bind _result (Math|Integer|IncrementInt (Variables|/Game/Blueprints/BP_Character.BP_Character_C|Getpopechurches _asbp_character))
        (:%20%20
          (Variables|/Game/Blueprints/BP_Character.BP_Character_C|Setpopechurches _asbp_character _result))))
    (:then_1
      (bind _returnvalue (Game|SpawnActorfromClass "/Game/Blueprints/AI/BP_Pope.BP_Pope_C" (Math|Transform|MakeTransform (+ (Transformation|GetWorldLocation _chathedral) (* (Math|Vector|GetForwardVector _chathedral) 300)) "0,180.000000, 0" "1,1,1") "AdjustIfPossibleButAlwaysSpawn" 0 0))
      (Variables|/Game/Blueprints/AI/BP_Pope.BP_Pope_C|SetPatrolPathBasilica _returnvalue self)
      (Development|PrintString "Hello"))))

(fn ConstructionScript
  (bind _returnvalue (Rendering|Material|CreateDynamicMaterialInstance (Variables|Default|GetChathedral) 0 0 "None" :!class /Script/Engine.PrimitiveComponent))
  (bind _output_get (Variables|Default|SetDynamicMaterial _returnvalue))
  (Rendering|Material|SetVectorParameterValue _output_get "Color" (Math|Color|MakeColor 0.0 1.0 0.0) :!class /Script/Engine.MaterialInstanceDynamic))