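; BP_Minion_Spawner is an actor that spawns BP_Minion at its own location about every two seconds.
; Tick drives the loop, with an IsSpawning flag blocking re-entry until the Delay finishes.
; Each spawn increments the Minions count in BPPersistantGameInstance, which also caps spawning at roughly 500.
; Once that cap check fails, the flag is never cleared, so this spawner stops permanently.
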(event EventBeginPlay)

(event Collision|EventActorBeginOverlap
  (params (OtherActor :type Actor%20Object%20Reference)))

(event EventTick
  (params (DeltaSeconds :type Float%20%28single-precision%29))
  (bind _bp_persistant_game_instance (Variables|Default|GetBP_Persistant_Game_Instance))
  (if (not (Variables|Default|GetisSpawning))
    (Variables|Default|SetisSpawning true)
    (if (<= (Variables|/Game/Blueprints/BP_Persistant_Game_Instance.BP_Persistant_Game_Instance_C|Getminions (Variables|Default|GetBP_Persistant_Game_Instance)) 500)
      (Variables|/Game/Blueprints/BP_Persistant_Game_Instance.BP_Persistant_Game_Instance_C|Setminions _bp_persistant_game_instance (+ (Variables|/Game/Blueprints/BP_Persistant_Game_Instance.BP_Persistant_Game_Instance_C|Getminions _bp_persistant_game_instance) 1))
      (Game|SpawnActorfromClass "/Game/Blueprints/AI/BP_Minion.BP_Minion_C" (Math|Transform|MakeTransform (Transformation|GetWorldLocation (Variables|Default|GetDefaultSceneRoot)) "0, 0, 0" "1,1,1") "AdjustIfPossibleButAlwaysSpawn" 0 0)
      (Utilities|FlowControl|Delay 2.0)
      (Variables|Default|SetisSpawning false))))

(fn ConstructionScript)