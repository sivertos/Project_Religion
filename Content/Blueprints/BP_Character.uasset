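; First-person player character for a religion game about gathering followers, building churches and performing miracles.
; Tick adds mana from church, cathedral and pope-church counts, throttled by a delay gate.
; A debug-key line trace to a church spawner places churches given enough followers; the card-trick miracle animates cards, then messages all "Human"-tagged actors.
; Also handles movement and HUD creation; click conversion and the wineglass miracle are unfinished.
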(event Custom|add%20mana
  ;[1 1 1] Adder mana basert på kirker + katedraler + pavekirker
  (if (not (Variables|Default|GetcountingMana))
    (Variables|Default|SetcountingMana true)
    (Variables|Default|Setmana (+ (Variables|Default|Getmana) (* (Variables|Default|Getchurches) (Variables|Default|GetchurchMana)) (* (Variables|Default|Getcathedrals) (Variables|Default|GetcathedralMana)) (* (Variables|Default|Getpopechurches) (Variables|Default|GetpopecurchMana))))
    (Utilities|FlowControl|Delay 1.0)
    (Variables|Default|SetcountingMana false)))

(event Custom|spawnChurch_1
  (for _index (range 1 (Variables|Default|GetchurchCost))
    (bind _result (Math|Integer|DecrementInt _index)
      (:%20%20
        (Actor|DestroyActor (Utilities|Array|Get(acopy) (Variables|Default|Getbelivers) _result))))))

(event EventBeginPlay
  (bind _returnvalue (UserInterface|CreateWidget "/Game/Blueprints/Widgets/BP_HUD.BP_HUD_C"))
  (bind _returnvalue_2 (Game|GetCurrentLevelName true))
  (if (not (Utilities|Enum|Equal(Enum) _returnvalue_2 "MainMenu"))
    (UserInterface|Viewport|AddtoViewport _returnvalue 0)))

(event Collision|EventActorBeginOverlap
  (params (OtherActor :type Actor%20Object%20Reference))
  (Variables|Default|SetbIsInRange true))

(event EventTick
  (params (DeltaSeconds :type Float%20%28single-precision%29))
  ;[1 1 1] Tick
  (CallFunction|AddMana))

(event Input|ActionEvents|InputActionJump
  (params (Key :type Key%20Structure :default "None"))
  ;[1 1 1] Jump binding
  (:Pressed
    (Character|Jump)))

(event Input|ActionEvents|InputActionAction4
  (params (Key :type Key%20Structure :default "None")))

(event Input|ActionEvents|InputActionAction5
  (params (Key :type Key%20Structure :default "None")))

(event Input|ActionEvents|InputActionMouseClick
  (params (Key :type Key%20Structure :default "None"))
  (bind _cameracomponent (Variables|Default|GetCameraComponent))
  (bind _returnvalue (Transformation|GetWorldLocation _cameracomponent))
  ;[1 1 1] Gjør convert funksjonen videre med victim som object reference
  (:Pressed
    (bind (_outhit _returnvalue_2) (Collision|LineTraceByChannel _returnvalue (+ _returnvalue (+ (Math|Vector|GetForwardVector _cameracomponent) 400)) "TraceTypeQuery1" false 0 "None"))
    (if _returnvalue_2
      (Utilities|Casting|CastToBP_Minion (.HitActor (Collision|BreakHitResult _outhit))))))

(event Input|ActionEvents|InputActionAction1
  (params (Key :type Key%20Structure :default "None"))
  (bind _card1 (Variables|Default|GetCard1))
  (bind _returnvalue (Transformation|GetWorldRotation _card1))
  (bind (_roll _pitch _yaw) (Math|Rotator|BreakRotator _returnvalue))
  ;[1 1 1] Mirakel 1: Korttriks
  (:Pressed
    (if (not (Variables|Default|GetdoingAction))
      (Variables|Default|SetdoingAction true)
      (Utilities|FlowControl|Sequence
        (:then_0
          (Rendering|SetVisibility (Variables|Default|GetCard1) true false))
        (:then_1
          (Rendering|SetVisibility (Variables|Default|GetCard2) true false))
        (:then_2
          (bind _returnvalue_2 (AddComponent|AddSphereComponent false (Math|Transform|MakeTransform "0, 0, 0" "0, 0, 0" "20.000000,20.000000,20.000000")))
          (Variables|Default|SetMiracle1%20CollisionSphere _returnvalue_2)
          (bind _newtrack_0 (Timeline|RotateCards PlayFromStart)
            (:Update
              (Transformation|SetWorldRotation _card1 (Math|Rotator|MakeRotator _newtrack_0 _pitch _yaw) false false))
            (:Finished
              (bind _outactors (Actor|GetAllActorswithTag "Human"))
              (for _array_element _outactors
                (Class|BPMiracleInterface|Miracle(Message) _array_element)
                (Utilities|FlowControl|Delay 1.0)
                (Rendering|SetVisibility (Variables|Default|GetCard1) false false)
                (Rendering|SetVisibility (Variables|Default|GetCard2) false false)
                (Components|DestroyComponent (Variables|Default|GetMiracle1%20CollisionSphere))
                (Variables|Default|SetdoingAction false)))))))))

(event Input|ActionEvents|InputActionAction2
  (params (Key :type Key%20Structure :default "None"))
  (:Pressed
    (if (not (Variables|Default|GetdoingAction))
      (Variables|Default|SetdoingAction true)
      (bind _returnvalue (AddComponent|AddStaticMeshComponent false))
      (Variables|Default|Setwineglass _returnvalue)
      (bind _returnvalue_2 (AddComponent|AddSphereComponent false (Math|Transform|MakeTransform "0, 0, 0" "0, 0, 0" "20.000000,20.000000,20.000000")))
      (Variables|Default|SetMiracle2%20CollisionSphere _returnvalue_2))))

(event Input|ActionEvents|InputActionAction3
  (params (Key :type Key%20Structure :default "None")))

(event Input|AxisEvents|InputAxisTurn
  (params (AxisValue :type Float%20%28single-precision%29))
  ;[1 1 1] Set up camera/mouse bindings
  (Pawn|Input|AddControllerYawInput AxisValue))

(event Input|AxisEvents|InputAxisLookUp
  (params (AxisValue :type Float%20%28single-precision%29))
  ;[1 1 1] Set up camera/mouse bindings
  (Pawn|Input|AddControllerPitchInput AxisValue))

(event Input|AxisEvents|InputAxisMoveForward
  (params (AxisValue :type Float%20%28single-precision%29))
  ;[1 1 1] Movement inputs
  (Pawn|Input|AddMovementInput (Math|Vector|GetForwardVector (Variables|Collision|GetCapsuleComponent)) AxisValue false))

(event Input|AxisEvents|InputAxisMoveRIght
  (params (AxisValue :type Float%20%28single-precision%29))
  ;[1 1 1] Movement inputs
  (Pawn|Input|AddMovementInput (Math|Vector|GetRightVector (Variables|Collision|GetCapsuleComponent)) AxisValue false))

(event Input|KeyboardEvents|9
  (params (Key :type Key%20Structure :default "None"))
  (:Pressed
    (bind _outactors (Actor|GetAllActorswithTag "Human"))
    (for _array_element _outactors
      (Class|BPMiracleInterface|Miracle(Message) _array_element))))

(event Input|KeyboardEvents|6
  (params (Key :type Key%20Structure :default "None"))
  ;[1 1 1] debug
  (:Pressed
    (for _array_element (Variables|Default|Getbelivers)
      (Development|PrintString (Utilities|GetDisplayName _array_element) true true "(R=0.000000,G=0.660000,B=1.000000,A=1.000000)" 5.0))))

(event Input|KeyboardEvents|5
  (params (Key :type Key%20Structure :default "None"))
  (bind _returnvalue (Class|Character|GetBaseRotationOffsetRotator))
  (bind _capsulecomponent (Variables|Collision|GetCapsuleComponent))
  (bind _cameracomponent (Variables|Default|GetCameraComponent))
  (bind _returnvalue_2 (Transformation|GetWorldLocation _capsulecomponent))
  (bind _returnvalue_3 (Math|Vector|GetForwardVector _capsulecomponent))
  (bind _returnvalue_4 (Transformation|GetWorldLocation _cameracomponent))
  (bind _returnvalue_5 (* _returnvalue_3 400))
  (bind _returnvalue_6 (+ _returnvalue_2 _returnvalue_5))
  (bind (_x _y) (Math|Vector|BreakVector _returnvalue_6))
  (:Pressed
    (bind (_outhit _returnvalue_7) (Collision|LineTraceByChannel _returnvalue_4 (+ _returnvalue_4 (* (Math|Vector|GetForwardVector _cameracomponent) 400)) "TraceTypeQuery1" false 0 "ForDuration"))
    (if _returnvalue_7
      (bind _asbp_church_spawner (Utilities|Casting|CastToBP_ChurchSpawner (.HitActor (Collision|BreakHitResult _outhit))))
      ;[1 1 1] Plasserer en kirke i levelet
      (if (>= (Variables|Default|Getfollowers) 5)
        (Class|BPMiracleInterface|SpawnChurch1(Message) _asbp_church_spawner)
        (Game|SpawnActorfromClass "/Game/Blueprints/BP_Church.BP_Church_C" (Math|Transform|MakeTransform (Math|Vector|MakeVector _x _y 221.0) (Math|Rotator|MakeRotator (.roll _returnvalue) (.pitch _returnvalue) (- (.yaw _returnvalue) 1.8e+02)) "1,1,1") "AdjustIfPossibleButDontSpawnIfColliding" 0 0)))))

(fn ConstructionScript)