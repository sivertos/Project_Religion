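; BP_Minion is an AI character that a Miracle event can convert into a believer following the player.
; Tick writes zone overlap to the Blackboard, plus a proximity flag for believers, while AI Perception writes player visibility.
; Miracle gives overlapping minions a random conversion chance, registering them with BP_Character, swapping material and incrementing the follower count.
; The Counted guard is never set true, so repeated conversions can count again.
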(event OnTargetPerceptionUpdated(AIPerception)
  (params (Actor :type Actor%20Object%20Reference) (Stimulus :type AI%20Stimulus%20Structure))
  (Utilities|Casting|CastToBP_Character Actor)
  (AI|Components|Blackboard|SetValueasBool (AI|GetBlackboard 0) (Utilities|Name|MakeLiteralName "canSeePlayer") (.bSuccessfullySensed (Utilities|Struct|BreakAIStimulus Stimulus))))

(event Custom|updateFollowers
  ;[1 1 1] Oppdaterer varibler som har med følgere, og oppdaterer modellene.
  (if (and (Variables|Default|GetBeliver) (Math|Boolean|NotEqual(Boolean) (Variables|Default|Getcounted) true))
    (Rendering|Material|SetMaterial (Variables|Default|Gethuman) 0 "/Game/Assets/Materials/beliber.beliber")
    (bind _asbp_character (Utilities|Casting|CastToBP_Character (Game|GetPlayerCharacter 0)))
    (bind _result (Math|Integer|IncrementInt (Variables|/Game/Blueprints/BP_Character.BP_Character_C|Getfollowers _asbp_character))
      (:%20%20
        (Variables|/Game/Blueprints/BP_Character.BP_Character_C|Setfollowers _asbp_character _result)
        (Variables|Default|Setcounted false)))))

(event Custom|set%20balckboard%20within%20zone
  (bind _returnvalue (Utilities|Name|MakeLiteralName "withinZone"))
  (bind _returnvalue_2 (AI|GetBlackboard 0))
  (bind _asbp_character (Utilities|Casting|CastToBP_Character (Game|GetPlayerCharacter 0)))
  (if (Collision|IsOverlappingActor _asbp_character :!class /Script/Engine.Actor)
    (AI|Components|Blackboard|SetValueasBool _returnvalue_2 _returnvalue true)
    (else
      (AI|Components|Blackboard|SetValueasBool _returnvalue_2 _returnvalue false))))

(event Custom|set%20blackboard%20within%20range
  (bind _returnvalue (Utilities|Name|MakeLiteralName "inRange"))
  (bind _returnvalue_2 (AI|GetBlackboard 0))
  (if (< (Math|Vector|VectorLength (- (Transformation|GetWorldLocation (Variables|Collision|GetCapsuleComponent)) (Transformation|GetWorldLocation (Variables|/Script/Engine.Character|GetCapsuleComponent (Game|GetPlayerCharacter 0))))) 3e+02)
    (AI|Components|Blackboard|SetValueasBool _returnvalue_2 _returnvalue true)
    (else
      (AI|Components|Blackboard|SetValueasBool _returnvalue_2 _returnvalue false))))

(event EventTick
  (params (DeltaSeconds :type Float%20%28single-precision%29))
  (CallFunction|SetBalckboardWithinZone)
  (if (Variables|Default|GetBeliver)
    (CallFunction|SetBlackboardWithinRange)))

(event EventMiracle
  (bind _asbp_character (Utilities|Casting|CastToBP_Character (Game|GetPlayerCharacter 0)))
  (if (Collision|IsOverlappingActor _asbp_character :!class /Script/Engine.Actor)
    (if (> (Math|Random|RandomIntegerinRange 1 10) 5)
      (Variables|Default|SetBeliver true)
      (Utilities|Array|Add (Variables|/Game/Blueprints/BP_Character.BP_Character_C|Getbelivers _asbp_character) self)
      (AI|Components|Blackboard|SetValueasBool (AI|GetBlackboard 0) (Utilities|Name|MakeLiteralName "beliver") true)
      (CallFunction|UpdateFollowers))))

(fn ConstructionScript)