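; BP_Pope is an AI priest character styled with the icon and color held in the persistent game instance.
; The construction script tints a dynamic material on the Priest component, and BeginPlay sets the selected icon as decal material.
; Perception updates set the blackboard's canSeePlayer true for any actor.
; For a BP_Minion, it also stores the reference and overwrites that flag with the sensed result.
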(event OnTargetPerceptionUpdated(AIPerception)
  (params (Actor :type Actor%20Object%20Reference) (Stimulus :type AI%20Stimulus%20Structure))
  (AI|Components|Blackboard|SetValueasBool (AI|GetBlackboard 0) (Utilities|Name|MakeLiteralName "canSeePlayer") true)
  (bind _asbp_minion (Utilities|Casting|CastToBP_Minion Actor))
  (Variables|Default|SetBP_Minion _asbp_minion)
  (AI|Components|Blackboard|SetValueasBool (AI|GetBlackboard 0) (Utilities|Name|MakeLiteralName "canSeePlayer") (.bSuccessfullySensed (Utilities|Struct|BreakAIStimulus Stimulus))))

(event EventBeginPlay
  (bind _asbp_persistant_game_instance (Utilities|Casting|CastToBP_Persistant_Game_Instance (Game|GetGameInstance)))
  (Rendering|Components|Decal|SetDecalMaterial (Variables|Default|GetDecal) (Utilities|Array|Get(acopy) (Variables|/Game/Blueprints/BP_Persistant_Game_Instance.BP_Persistant_Game_Instance_C|GetIcon _asbp_persistant_game_instance) (Variables|/Game/Blueprints/BP_Persistant_Game_Instance.BP_Persistant_Game_Instance_C|Getselected%20icon _asbp_persistant_game_instance))))

(event Collision|EventActorBeginOverlap
  (params (OtherActor :type Actor%20Object%20Reference)))

(event EventTick
  (params (DeltaSeconds :type Float%20%28single-precision%29)))

(fn ConstructionScript
  (bind _returnvalue (Rendering|Material|CreateDynamicMaterialInstance (Variables|Default|Getpriest) 0 0 "None" :!class /Script/Engine.PrimitiveComponent))
  (bind _output_get (Variables|Default|SetDynamicMaterial _returnvalue))
  (bind _asbp_persistant_game_instance (Utilities|Casting|CastToBP_Persistant_Game_Instance (Game|GetGameInstance)))
  (Rendering|Material|SetVectorParameterValue _output_get "Color" (Variables|/Game/Blueprints/BP_Persistant_Game_Instance.BP_Persistant_Game_Instance_C|GetRelColor _asbp_persistant_game_instance) :!class /Script/Engine.MaterialInstanceDynamic))