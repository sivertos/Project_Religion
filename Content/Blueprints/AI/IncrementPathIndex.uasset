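; Behavior Tree task that advances the patrol waypoint index for a BP_Priest pawn.
; It increments the blackboard path index, wrapping to zero after the last entry in the priest's PatrolPathCurch PathVectors to loop the patrol.
; It finishes successfully after the update, but a failed cast to BP_Priest stops execution without calling FinishExecute.
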(event EventReceiveExecuteAI
  (params (OwnerController :type AI%20Controller%20Object%20Reference) (ControlledPawn :type Pawn%20Object%20Reference))
  (bind _bb_pathindex (Variables|Default|GetBB_pathIndex))
  (bind _returnvalue (Class|BTFunctionLibrary|GetBlackboardValueasInt _bb_pathindex))
  (bind _returnvalue_2 (+ _returnvalue 1))
  (bind _asbp_priest (Utilities|Casting|CastToBP_Priest ControlledPawn))
  (if (<= _returnvalue_2 (- (Utilities|Array|Length (Variables|/Game/Blueprints/BP_Church.BP_Church_C|GetpathVectors (Variables|/Game/Blueprints/AI/BP_Priest.BP_Priest_C|GetPatrolPathCurch _asbp_priest))) 1))
    (Class|BTFunctionLibrary|SetBlackboardValueasInt (Variables|Default|GetBB_pathIndex) _returnvalue_2)
    (else
      (Class|BTFunctionLibrary|SetBlackboardValueasInt (Variables|Default|GetBB_pathIndex))))
  (AI|BehaviorTree|FinishExecute true))