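; Behavior Tree task that picks a follow destination near the player for an AI.
; On execute, it casts player 0's pawn to BP_Character and finds a random reachable navmesh point within a small fixed radius of its mesh location.
; It writes that point to a Vector blackboard key and finishes successfully without checking the query result.
; A failed cast leaves the task unfinished.
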(event EventReceiveExecuteAI
  (params (OwnerController :type AI%20Controller%20Object%20Reference) (ControlledPawn :type Pawn%20Object%20Reference))
  (bind _asbp_character (Utilities|Casting|CastToBP_Character (Game|GetPlayerCharacter 0)))
  (AI|BehaviorTree|SetBlackboardValueasVector (Variables|Default|Getvector) (.RandomLocation (AI|Navigation|GetRandomReachablePointinRadius (Transformation|GetWorldLocation (Variables|/Script/Engine.Character|GetMesh _asbp_character)) 4e+01 0 0)))
  (AI|BehaviorTree|FinishExecute true))