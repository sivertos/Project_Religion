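; Behavior tree task that gives the Priest AI its next point on its church patrol path.
; It reads the path index from the blackboard, picks that entry in the PathVectors of the priest's PatrolPathCurch actor, and adds the actor's location, ignoring rotation and scale.
; The result goes to the path vector key and the task succeeds; with a failed cast or invalid path, it never calls FinishExecute.
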(event EventReceiveExecuteAI
  (params (OwnerController :type AI%20Controller%20Object%20Reference) (ControlledPawn :type Pawn%20Object%20Reference))
  (bind _asbp_priest (Utilities|Casting|CastToBP_Priest ControlledPawn))
  (bind _patrolpathcurch (Variables|/Game/Blueprints/AI/BP_Priest.BP_Priest_C|GetPatrolPathCurch _asbp_priest)
    (:then
      (AI|BehaviorTree|SetBlackboardValueasVector (Variables|Default|GetBB_PathVector) (+ (.location (Transformation|GetActorTransform _patrolpathcurch)) (Utilities|Array|Get(acopy) (Variables|/Game/Blueprints/BP_Church.BP_Church_C|GetpathVectors _patrolpathcurch) (Class|BTFunctionLibrary|GetBlackboardValueasInt (Variables|Default|GetBB_PathIndex)))))
      (AI|BehaviorTree|FinishExecute true))
    (:else)))