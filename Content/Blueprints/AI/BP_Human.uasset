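; BP_Human is a human actor that the player can convert into a believer, adding to their follower count.
; When the Miracle event fires while the player character overlaps it, a random roll gives an even chance of setting the believer flag.
; UpdateFollowers then swaps the human's material and increments Followers on BP_Character, with a Counted flag ensuring each human counts only once.
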(event Custom|updateFollowers
  (if (and (Variables|Default|GetBeliver) (Math|Boolean|NotEqual(Boolean) (Variables|Default|Getcounted) true))
    (Rendering|Material|SetMaterial (Variables|Default|GetHuman) 0 "/Game/Assets/Materials/beliber.beliber")
    (bind _asbp_character (Utilities|Casting|CastToBP_Character (Game|GetPlayerCharacter 0)))
    (bind _result (Math|Integer|IncrementInt (Variables|/Game/Blueprints/BP_Character.BP_Character_C|Getfollowers _asbp_character))
      (:%20%20
        (Variables|/Game/Blueprints/BP_Character.BP_Character_C|Setfollowers _asbp_character _result)
        (Variables|Default|Setcounted true)))))

(event EventBeginPlay)

(event Collision|EventActorBeginOverlap
  (params (OtherActor :type Actor%20Object%20Reference)))

(event EventMiracle
  (bind _asbp_character (Utilities|Casting|CastToBP_Character (Game|GetPlayerCharacter 0)))
  (if (Collision|IsOverlappingActor _asbp_character :!class /Script/Engine.Actor)
    (if (> (Math|Random|RandomIntegerinRange 1 10) 5)
      (Variables|Default|SetBeliver true)
      (CallFunction|UpdateFollowers))))

(event EventTick
  (params (DeltaSeconds :type Float%20%28single-precision%29)))

(fn ConstructionScript)