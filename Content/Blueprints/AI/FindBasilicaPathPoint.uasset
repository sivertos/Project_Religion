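; Behavior tree task that picks the next Basilica patrol destination for BP_Pope.
; It reads the blackboard path index, looks up that offset in the Pope's PatrolPathBasilica vectors and adds it to his current location.
; The result is written to the blackboard path vector and the task succeeds; a failed cast never finishes the task.
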(event EventReceiveExecuteAI
  (params (OwnerController :type AI%20Controller%20Object%20Reference) (ControlledPawn :type Pawn%20Object%20Reference))
  (bind _asbp_pope (Utilities|Casting|CastToBP_Pope ControlledPawn))
  (AI|BehaviorTree|SetBlackboardValueasVector (Variables|Default|GetBB_PathVector) (+ (.location (Transformation|GetActorTransform _asbp_pope)) (Utilities|Array|Get(acopy) (Variables|/Game/Blueprints/BP_Basilica.BP_Basilica_C|GetpathVectors (Variables|/Game/Blueprints/AI/BP_Pope.BP_Pope_C|GetPatrolPathBasilica _asbp_pope)) (Class|BTFunctionLibrary|GetBlackboardValueasInt (Variables|Default|GetBB_PathIndex)))))
  (AI|BehaviorTree|FinishExecute true))