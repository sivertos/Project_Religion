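; FindCathedralPathPoint is a Behavior Tree task that picks a patrol destination for the Bishop AI on its cathedral path.
; It reads the path index from the Blackboard and looks up that entry in the path vectors of the Bishop's PatrolPathCathedral.
; It adds the entry to the Bishop's current location, writes the result to the path vector key and finishes successfully, leaving the index unchanged.
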(event EventReceiveExecuteAI
  (params (OwnerController :type AI%20Controller%20Object%20Reference) (ControlledPawn :type Pawn%20Object%20Reference))
  (bind _asbp_bishop (Utilities|Casting|CastToBP_Bishop ControlledPawn))
  (AI|BehaviorTree|SetBlackboardValueasVector (Variables|Default|GetBB_PathVector) (+ (.location (Transformation|GetActorTransform _asbp_bishop)) (Utilities|Array|Get(acopy) (Variables|/Game/Blueprints/BP_Cathedral.BP_Cathedral_C|GetpathVectors (Variables|/Game/Blueprints/AI/BP_Bishop.BP_Bishop_C|GetPatrolPathCathedral _asbp_bishop)) (Class|BTFunctionLibrary|GetBlackboardValueasInt (Variables|Default|GetBB_PathIndex)))))
  (AI|BehaviorTree|FinishExecute true))