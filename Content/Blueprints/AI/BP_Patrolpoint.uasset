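; BP_Patrolpoint is an AI patrol-point Blueprint that turns four placed Box components into a list of patrol locations.
; On BeginPlay it gathers the components into a Boxes array, then stores each one's world location in the Patrolpoints array.
; The locations are captured once at startup, and this Blueprint contains no movement logic of its own.
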(event EventBeginPlay
  (bind _boxes (Variables|Default|GetBoxes))
  (Utilities|FlowControl|Sequence
    (:then_0
      (Utilities|Array|Add _boxes (Variables|Default|GetBox)))
    (:then_1
      (Utilities|Array|Add _boxes (Variables|Default|GetBox1)))
    (:then_2
      (Utilities|Array|Add _boxes (Variables|Default|GetBox2)))
    (:then_3
      (Utilities|Array|Add _boxes (Variables|Default|GetBox3)))
    (:then_4
      (for _array_element (Variables|Default|GetBoxes)
        (Utilities|Array|Add (Variables|Default|GetPatrolpoints) (Transformation|GetWorldLocation _array_element))))))

(fn ConstructionScript)